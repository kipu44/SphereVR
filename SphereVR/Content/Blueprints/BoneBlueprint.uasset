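; Leap Motion hand bone Blueprint that acts as a debug prototype for tracking fingertip position.
; On Tick, the index fingertip bone stores its offset from the player character in FingerLocation and prints it, with the movement threshold bypassed.
; Disconnected node chains hold unfinished experiments for thumb tracking, value caching and a finger-to-thumb proximity "magic" pinch check, none of which run.
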(event `self.ReceiveTick`
  (params (DeltaSeconds :type "Float (single-precision)"))
  (bind _returnvalue (- (`self.K2_GetActorLocation` (`GameplayStatics.GetPlayerCharacter` 0)) (`self.K2_GetActorLocation`)))
  (bind _returnvalue_2 (- _returnvalue (`self.FingerLocation`)))
  (if false
    (`KismetSystemLibrary.PrintString` "Bone Event Graph"))
  (if true
    ;[1 1 1] finger
    (if (`|EnumEquality` (`self.LeapBoneType`) "Finger1Tip")
      (if (or (> (`KismetMathLibrary.VSizeSquared` _returnvalue_2) 3000.0) true)
        (`KismetSystemLibrary.PrintString` (`KismetStringLibrary.Concat_StrStr` "      B         move: " (`KismetStringLibrary.Conv_VectorToString` _returnvalue_2)))
        (bind _output_get (set `self.FingerLocation` _returnvalue))
        (if true
          (`KismetSystemLibrary.PrintString` (`KismetStringLibrary.Concat_StrStr` "      B         finger: " (`KismetStringLibrary.Conv_VectorToString` _output_get))))
        (if true :!label _label
          _))
      (else
        (goto _label)))))

(fn `UserConstructionScript`)