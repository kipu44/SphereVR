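; Leap Motion hand Blueprint that poses a rigged hand mesh from physical per-bone actors.
; Tick mirrors the left hand by negative scale, places the mesh at the computed elbow and copies bone-actor rotations with rig-basis offsets.
; The construction script fills the rig bone names from a delimited string.
; An unfinished, print-only thumb-to-finger pinch check reads the hand actor's own location for both tips, not the bones'.
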(event EventTick
  (params (DeltaSeconds :type Float%20%28single-precision%29))
  (bind _returnvalue (Class|LeapMotionHandActor|GetBoneActor "Forearm"))
  (bind _handid (Variables|Default|GetHandId))
  (bind _fingerlocation (Variables|Default|GetFingerLocation))
  (bind _scale (Variables|Default|GetScale))
  (bind _handside (Variables|Default|GetHandSide))
  (bind _outlength (Class|LeapMotionFunctionLibrary|GetBoneWidthandLength _handid "Forearm"))
  (bind _returnvalue_2 (Transformation|GetActorRotation _returnvalue))
  (bind _returnvalue_3 (Transformation|GetActorLocation _returnvalue))
  (bind _returnvalue_4 (Utilities|Enum|Equal(Enum) _handside "Left"))
  (bind _returnvalue_5 (Math|Float|SelectFloat 1.0 -1.0 _returnvalue_4))
  (bind _returnvalue_6 (Math|Rotator|SelectRotator "0,90.000000,180.000000" "0.000000,90.000000,0.000000" _returnvalue_4))
  (bind _returnvalue_7 (Math|Rotator|CombineRotators _returnvalue_6 _returnvalue_2))
  (bind _returnvalue_8 (* _scale _returnvalue_5))
  (bind _returnvalue_9 (* _outlength _returnvalue_8))
  (bind _returnvalue_10 (Math|Vector|MakeVector 0.0 0.0 _returnvalue_9))
  (bind _returnvalue_11 (Math|Vector|RotateVector _returnvalue_10 _returnvalue_7))
  (bind _returnvalue_12 (+ _returnvalue_3 _returnvalue_11))
  (Utilities|FlowControl|Sequence
    (:then_0
      (if true
        (Utilities|FlowControl|DoOnce false
          (:Completed
            ;[1 1 1] Match scale of the physical representation
            (Transformation|SetRelativeScale3D (Math|Conversions|ToVector(Float) (* (Math|Float|SelectFloat -1.0 1.0 _returnvalue_4) (Variables|Default|GetScale))))))))
    (:then_1
      (Development|PrintString (Utilities|String|Append "new location: " (Utilities|String|ToString(Vector) _returnvalue_12)))
      (if true
        (Transformation|SetWorldLocation _returnvalue_12 false)
        ;[1 1 1] Set global rotation of each bone. Rig bones are referred by names, which are manually stored in Rig Bone Names in the Construction Script.
        (if true
          (bind _enumvalue (|ForEachELeapBone)
            (:LoopBody
              (Components|PoseableMesh|SetBoneRotationbyName (Utilities|Array|Get(acopy) (Variables|Default|GetRigBoneNames) (Math|Conversions|ToInteger(Byte) _enumvalue)) (Math|Rotator|CombineRotators (Math|Rotator|CombineRotators (Math|Rotator|SelectRotator "90.000000,180.000000, 0" "90.000000,90.000000, 0" (Utilities|Enum|Equal(Enum) _enumvalue "Forearm")) (Math|Rotator|SelectRotator "180.000000,0.000000,0.000000" "0.000000,0.000000,0.000000" _returnvalue_4)) (Transformation|GetActorRotation (Class|LeapMotionHandActor|GetBoneActor _enumvalue))) "WorldSpace"))))))
    (:then_2
      (if true
        (Development|PrintString "     H foreach"))
      (Variables|Default|Setboth false)
      (Development|PrintString (Utilities|String|Append "1 both: " (Utilities|String|ToString(Boolean) (Variables|Default|Getboth))))
      (bind _enumvalue_2 (|ForEachELeapBone)
        (:LoopBody
          (if true
            ;[1 1 1] finger
            (if (Utilities|Enum|Equal(Enum) _enumvalue_2 "Finger1Tip")
              (Variables|Default|Setboth (or (Utilities|Enum|Equal(Enum) _enumvalue_2 "Finger1Tip") (Variables|Default|Getboth)))
              (bind _output_get (Variables|Default|SetfingerLocation (Transformation|GetActorLocation)))
              (Development|PrintString (Utilities|String|Append " finger: " (Utilities|String|ToString(Vector) _output_get))))
            (if true
              (if true
                ;[1 1 1] thumb
                (if (Utilities|Enum|Equal(Enum) _enumvalue_2 "ThumbTip")
                  (Variables|Default|Setboth (or (Utilities|Enum|Equal(Enum) _enumvalue_2 "ThumbTip") (Variables|Default|Getboth)))
                  (Development|PrintString (Utilities|String|Append "2 both: " (Utilities|String|ToString(Boolean) (Variables|Default|Getboth))))
                  (bind _output_get_2 (Variables|Default|SetThumbLocation (Transformation|GetActorLocation)))
                  (Development|PrintString (Utilities|String|Append "thumb: " (Utilities|String|ToString(Vector) _output_get_2))))
                (if true
                  _)))))
        (:then
          (Development|PrintString (Utilities|String|Append "3 both: " (Utilities|String|ToString(Boolean) (Variables|Default|Getboth))))
          (if (Variables|Default|Getboth)
            ;[1 1 1] diff
            (Development|PrintString (Utilities|String|Append "D finger: " (Utilities|String|ToString(Vector) _fingerlocation)))
            (Development|PrintString (Utilities|String|Append "D thumb: " (Utilities|String|ToString(Vector) (Variables|Default|GetThumbLocation))))
            (Development|PrintString (Utilities|String|Append "      diff: " (Utilities|String|ToString(Vector) (- _fingerlocation (Variables|Default|GetThumbLocation)))))
            (if (< (Math|Vector|VectorLengthSquared (- _fingerlocation (Variables|Default|GetThumbLocation))) 1e+03)
              (Development|PrintString (Utilities|String|Append "magic! " (Utilities|String|ToString(Float) (Math|Vector|VectorLengthSquared (- _fingerlocation (Variables|Default|GetThumbLocation)))))))
            (if true
              _)))))))

(fn ConstructionScript
  (LocalVariables|SetTmpNames (Utilities|String|MakeLiteralString "Bip01-R-Forearm; Bip01-R-Hand; Bip01-R-Finger0; Bip01-R-Finger01; Bip01-R-Finger02; Bip01-R-Finger1; Bip01-R-Finger11; Bip01-R-Finger12; Bip01-R-Finger2; Bip01-R-Finger21; Bip01-R-Finger22; Bip01-R-Finger3; Bip01-R-Finger31; Bip01-R-Finger32; Bip01-R-Finger4; Bip01-R-Finger41; Bip01-R-Finger42; fin"))
  (while (Utilities|Enum|NotEqual(Enum) (LocalVariables|GetTmpNames) "fin")
    (Utilities|Array|Add (Variables|Default|GetRigBoneNames) (Utilities|String|StringToName (.LeftS (Utilities|String|Split (LocalVariables|GetTmpNames) "; "))))
    (LocalVariables|SetTmpNames (.RightS (Utilities|String|Split (LocalVariables|GetTmpNames) "; ")))))