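; Balance board controller Blueprint that turns a player's weight distribution into on/off forward, left and right inputs.
; Weight events store the four corner readings and the total, with debug float prints switched off, while BeginPlay and every Tick print "Hello".
; Getters require a minimum total, then compare weight shares against a threshold: front pair for forward, opposite diagonals for left and right.
; Only left also requires both its corners to outweigh the others.
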(event `self.TopRightWeightEvent`
  (params (weight :type "Float (single-precision)"))
  (bind _output_get (set `self.TopRight` weight))
  (`/Game/FirstPersonBP/Blueprints/PrintLibrary.printFloat` false "TRL" _output_get))

(event `self.TopLeftWeightEvent`
  (params (weight :type "Float (single-precision)"))
  (bind _output_get (set `self.TopLeft` weight))
  (`/Game/FirstPersonBP/Blueprints/PrintLibrary.printFloat` false "TLW" _output_get))

(event `self.BottomRightWeightEvent`
  (params (weight :type "Float (single-precision)"))
  (bind _output_get (set `self.BottomRight` weight))
  (`/Game/FirstPersonBP/Blueprints/PrintLibrary.printFloat` false "BRW" _output_get))

(event `self.BottomLeftWeightEvent`
  (params (weight :type "Float (single-precision)"))
  (bind _output_get (set `self.BottomLeft` weight))
  (`/Game/FirstPersonBP/Blueprints/PrintLibrary.printFloat` false "BLW" _output_get))

(event `self.TotalWeightEvent`
  (params (weight :type "Float (single-precision)"))
  (bind _output_get (set `self.Total` weight))
  (`/Game/FirstPersonBP/Blueprints/PrintLibrary.printFloat` false "Total" _output_get))

(event `self.ReceiveActorBeginOverlap`
  (params (OtherActor :type "Actor Object Reference")))

(event `self.ReceiveBeginPlay`
  (`KismetSystemLibrary.PrintString` "Hello" :!label _label))

(event `self.ReceiveTick`
  (params (DeltaSeconds :type "Float (single-precision)"))
  (goto _label))

(fn `GetForward`
  (returns (Output :type "Float (double-precision)"))
  (bind _total (`self.Total`))
  (if (> _total 10.0)
    (if (> (/ (+ (`self.TopLeft`) (`self.TopRight`)) _total) 0.55)
      (set `self.Direction` 1.0)
      (else
        (set `self.Direction` 0.0 :!label _label)))
    (else
      (goto _label)))
  (return (`self.Direction`)))

(fn `GetLeft`
  (returns (left :type "Float (double-precision)"))
  (bind _total (`self.Total`))
  (bind _topleft (`self.TopLeft`))
  (bind _bottomright (`self.BottomRight`))
  (bind _bottomleft (`self.BottomLeft`))
  (bind _topright (`self.TopRight`))
  (if (> _total 10.0)
    (if (and (> _topleft _bottomleft) (> _topleft _topright) (> _bottomright _topright) (> _bottomright _bottomleft) (> (/ (+ _topleft _bottomright) _total) 0.55))
      (set `self.Left` 1.0)
      (else
        (set `self.Left` 0.0 :!label _label)))
    (else
      (goto _label)))
  (return (`self.Left`)))

(fn `GetRight`
  (returns (right :type "Float (double-precision)"))
  (bind _total (`self.Total`))
  (if (> _total 10.0)
    (if (> (/ (+ (`self.TopRight`) (`self.BottomLeft`)) _total) 0.55)
      (set `self.Right` 1.0)
      (else
        (set `self.Right` 0.0 :!label _label)))
    (else
      (goto _label)))
  (return (`self.Right`)))

(fn `UserConstructionScript`)